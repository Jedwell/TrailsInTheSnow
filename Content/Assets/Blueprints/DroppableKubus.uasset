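; DroppableKubus is a hexagonal block that the ThirdPersonCharacter shoves in six directions, with R teleporting it back to its saved start transform.
; Side trigger boxes flag the shove direction, while check boxes flag obstacles so a shove is skipped if the opposite side is blocked.
; A DoOnce, reset when the character leaves, gates shoves that briefly enable physics and apply force.
; Touching DeletePhysics from below sets Drop, which this graph never reads.
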(event OnComponentBeginOverlap(BoxTopRight)
  (params (OverlappedComponent :type Primitive%20Component%20Object%20Reference) (OtherActor :type Actor%20Object%20Reference) (OtherComp :type Primitive%20Component%20Object%20Reference) (OtherBodyIndex :type Integer) (bFromSweep :type Boolean) (SweepResult :type Hit%20Result%20Structure%20%28by%20ref%29))
  (Utilities|Casting|CastToThirdPersonCharacter OtherActor)
  (Variables|Default|SetShoveTopRight true))

(event OnComponentBeginOverlap(BoxUp)
  (params (OverlappedComponent :type Primitive%20Component%20Object%20Reference) (OtherActor :type Actor%20Object%20Reference) (OtherComp :type Primitive%20Component%20Object%20Reference) (OtherBodyIndex :type Integer) (bFromSweep :type Boolean) (SweepResult :type Hit%20Result%20Structure%20%28by%20ref%29))
  (Utilities|Casting|CastToThirdPersonCharacter OtherActor)
  (Variables|Default|SetShoveUp true))

(event OnComponentBeginOverlap(BoxBottomLeft)
  (params (OverlappedComponent :type Primitive%20Component%20Object%20Reference) (OtherActor :type Actor%20Object%20Reference) (OtherComp :type Primitive%20Component%20Object%20Reference) (OtherBodyIndex :type Integer) (bFromSweep :type Boolean) (SweepResult :type Hit%20Result%20Structure%20%28by%20ref%29))
  (Utilities|Casting|CastToThirdPersonCharacter OtherActor)
  (Variables|Default|SetShoveBottomLeft true))

(event OnComponentEndOverlap(BoxBottomLeft)
  (params (OverlappedComponent :type Primitive%20Component%20Object%20Reference) (OtherActor :type Actor%20Object%20Reference) (OtherComp :type Primitive%20Component%20Object%20Reference) (OtherBodyIndex :type Integer))
  (bind _hexagon (Variables|Default|GetHexagon))
  (bind _hexagon_2 (Variables|Default|GetHexagon))
  (bind _hexagon_3 (Variables|Default|GetHexagon))
  (bind _hexagon_4 (Variables|Default|GetHexagon))
  (bind _hexagon_5 (Variables|Default|GetHexagon))
  (bind _hexagon_6 (Variables|Default|GetHexagon))
  (Utilities|Casting|CastToThirdPersonCharacter OtherActor)
  (Variables|Default|SetShoveBottomLeft false)
  (Utilities|FlowControl|DoOnce false) ; enters at Reset
)

(event OnComponentBeginOverlap(BoxCheckTopRight)
  (params (OverlappedComponent :type Primitive%20Component%20Object%20Reference) (OtherActor :type Actor%20Object%20Reference) (OtherComp :type Primitive%20Component%20Object%20Reference) (OtherBodyIndex :type Integer) (bFromSweep :type Boolean) (SweepResult :type Hit%20Result%20Structure%20%28by%20ref%29))
  (Utilities|Casting|CastToThirdPersonCharacter OtherActor
    (:CastFailed
      (Variables|Default|SetTopRightBlocked true))))

(event OnComponentEndOverlap(BoxCheckTopRight)
  (params (OverlappedComponent :type Primitive%20Component%20Object%20Reference) (OtherActor :type Actor%20Object%20Reference) (OtherComp :type Primitive%20Component%20Object%20Reference) (OtherBodyIndex :type Integer))
  (Utilities|Casting|CastToThirdPersonCharacter OtherActor
    (:CastFailed
      (Variables|Default|SetTopRightBlocked false))))

(event OnComponentBeginOverlap(BoxCheckUp)
  (params (OverlappedComponent :type Primitive%20Component%20Object%20Reference) (OtherActor :type Actor%20Object%20Reference) (OtherComp :type Primitive%20Component%20Object%20Reference) (OtherBodyIndex :type Integer) (bFromSweep :type Boolean) (SweepResult :type Hit%20Result%20Structure%20%28by%20ref%29))
  (Utilities|Casting|CastToThirdPersonCharacter OtherActor
    (:CastFailed
      (Variables|Default|SetUpBlocked true))))

(event OnComponentEndOverlap(BoxCheckUp)
  (params (OverlappedComponent :type Primitive%20Component%20Object%20Reference) (OtherActor :type Actor%20Object%20Reference) (OtherComp :type Primitive%20Component%20Object%20Reference) (OtherBodyIndex :type Integer))
  (Utilities|Casting|CastToThirdPersonCharacter OtherActor
    (:CastFailed
      (Variables|Default|SetUpBlocked false))))

(event OnComponentBeginOverlap(BoxCheckDown)
  (params (OverlappedComponent :type Primitive%20Component%20Object%20Reference) (OtherActor :type Actor%20Object%20Reference) (OtherComp :type Primitive%20Component%20Object%20Reference) (OtherBodyIndex :type Integer) (bFromSweep :type Boolean) (SweepResult :type Hit%20Result%20Structure%20%28by%20ref%29))
  (Utilities|Casting|CastToThirdPersonCharacter OtherActor
    (:CastFailed
      (Variables|Default|SetDownBlocked true))))

(event OnComponentEndOverlap(BoxCheckDown)
  (params (OverlappedComponent :type Primitive%20Component%20Object%20Reference) (OtherActor :type Actor%20Object%20Reference) (OtherComp :type Primitive%20Component%20Object%20Reference) (OtherBodyIndex :type Integer))
  (Utilities|Casting|CastToThirdPersonCharacter OtherActor
    (:CastFailed
      (Variables|Default|SetDownBlocked false))))

(event OnComponentBeginOverlap(BoxCheckTopLeft)
  (params (OverlappedComponent :type Primitive%20Component%20Object%20Reference) (OtherActor :type Actor%20Object%20Reference) (OtherComp :type Primitive%20Component%20Object%20Reference) (OtherBodyIndex :type Integer) (bFromSweep :type Boolean) (SweepResult :type Hit%20Result%20Structure%20%28by%20ref%29))
  (Utilities|Casting|CastToThirdPersonCharacter OtherActor
    (:CastFailed
      (Variables|Default|SetTopLeftBlocked true))))

(event OnComponentEndOverlap(BoxCheckTopLeft)
  (params (OverlappedComponent :type Primitive%20Component%20Object%20Reference) (OtherActor :type Actor%20Object%20Reference) (OtherComp :type Primitive%20Component%20Object%20Reference) (OtherBodyIndex :type Integer))
  (Utilities|Casting|CastToThirdPersonCharacter OtherActor
    (:CastFailed
      (Variables|Default|SetTopLeftBlocked false))))

(event OnComponentEndOverlap(BoxTopRight)
  (params (OverlappedComponent :type Primitive%20Component%20Object%20Reference) (OtherActor :type Actor%20Object%20Reference) (OtherComp :type Primitive%20Component%20Object%20Reference) (OtherBodyIndex :type Integer))
  (bind _hexagon (Variables|Default|GetHexagon))
  (bind _hexagon_2 (Variables|Default|GetHexagon))
  (bind _hexagon_3 (Variables|Default|GetHexagon))
  (bind _hexagon_4 (Variables|Default|GetHexagon))
  (bind _hexagon_5 (Variables|Default|GetHexagon))
  (bind _hexagon_6 (Variables|Default|GetHexagon))
  (Utilities|Casting|CastToThirdPersonCharacter OtherActor)
  (Variables|Default|SetShoveTopRight false)
  (Utilities|FlowControl|DoOnce false) ; enters at Reset
)

(event OnComponentBeginOverlap(BoxCheckBottomLeft)
  (params (OverlappedComponent :type Primitive%20Component%20Object%20Reference) (OtherActor :type Actor%20Object%20Reference) (OtherComp :type Primitive%20Component%20Object%20Reference) (OtherBodyIndex :type Integer) (bFromSweep :type Boolean) (SweepResult :type Hit%20Result%20Structure%20%28by%20ref%29))
  (Utilities|Casting|CastToThirdPersonCharacter OtherActor
    (:CastFailed
      (Variables|Default|SetBottomLeftBlocked true))))

(event OnComponentEndOverlap(BoxCheckBottomLeft)
  (params (OverlappedComponent :type Primitive%20Component%20Object%20Reference) (OtherActor :type Actor%20Object%20Reference) (OtherComp :type Primitive%20Component%20Object%20Reference) (OtherBodyIndex :type Integer))
  (Utilities|Casting|CastToThirdPersonCharacter OtherActor
    (:CastFailed
      (Variables|Default|SetBottomLeftBlocked false))))

(event OnComponentBeginOverlap(BoxCheckBottomRight)
  (params (OverlappedComponent :type Primitive%20Component%20Object%20Reference) (OtherActor :type Actor%20Object%20Reference) (OtherComp :type Primitive%20Component%20Object%20Reference) (OtherBodyIndex :type Integer) (bFromSweep :type Boolean) (SweepResult :type Hit%20Result%20Structure%20%28by%20ref%29))
  (Utilities|Casting|CastToThirdPersonCharacter OtherActor
    (:CastFailed
      (Variables|Default|SetBottomRightBlocked true))))

(event OnComponentEndOverlap(BoxCheckBottomRight)
  (params (OverlappedComponent :type Primitive%20Component%20Object%20Reference) (OtherActor :type Actor%20Object%20Reference) (OtherComp :type Primitive%20Component%20Object%20Reference) (OtherBodyIndex :type Integer))
  (Utilities|Casting|CastToThirdPersonCharacter OtherActor
    (:CastFailed
      (Variables|Default|SetBottomRightBlocked false))))

(event OnComponentBeginOverlap(Below)
  (params (OverlappedComponent :type Primitive%20Component%20Object%20Reference) (OtherActor :type Actor%20Object%20Reference) (OtherComp :type Primitive%20Component%20Object%20Reference) (OtherBodyIndex :type Integer) (bFromSweep :type Boolean) (SweepResult :type Hit%20Result%20Structure%20%28by%20ref%29))
  (Utilities|Casting|CastToDeletePhysics OtherActor)
  (Variables|Default|Setdrop true))

(event OnComponentEndOverlap(BoxUp)
  (params (OverlappedComponent :type Primitive%20Component%20Object%20Reference) (OtherActor :type Actor%20Object%20Reference) (OtherComp :type Primitive%20Component%20Object%20Reference) (OtherBodyIndex :type Integer))
  (bind _hexagon (Variables|Default|GetHexagon))
  (bind _hexagon_2 (Variables|Default|GetHexagon))
  (bind _hexagon_3 (Variables|Default|GetHexagon))
  (bind _hexagon_4 (Variables|Default|GetHexagon))
  (bind _hexagon_5 (Variables|Default|GetHexagon))
  (bind _hexagon_6 (Variables|Default|GetHexagon))
  (Utilities|Casting|CastToThirdPersonCharacter OtherActor)
  (Variables|Default|SetShoveUp false)
  (Utilities|FlowControl|DoOnce false) ; enters at Reset
)

(event OnComponentBeginOverlap(BoxBottomRight)
  (params (OverlappedComponent :type Primitive%20Component%20Object%20Reference) (OtherActor :type Actor%20Object%20Reference) (OtherComp :type Primitive%20Component%20Object%20Reference) (OtherBodyIndex :type Integer) (bFromSweep :type Boolean) (SweepResult :type Hit%20Result%20Structure%20%28by%20ref%29))
  (Utilities|Casting|CastToThirdPersonCharacter OtherActor)
  (Variables|Default|SetShoveBottomRight true))

(event OnComponentEndOverlap(BoxBottomRight)
  (params (OverlappedComponent :type Primitive%20Component%20Object%20Reference) (OtherActor :type Actor%20Object%20Reference) (OtherComp :type Primitive%20Component%20Object%20Reference) (OtherBodyIndex :type Integer))
  (bind _hexagon (Variables|Default|GetHexagon))
  (bind _hexagon_2 (Variables|Default|GetHexagon))
  (bind _hexagon_3 (Variables|Default|GetHexagon))
  (bind _hexagon_4 (Variables|Default|GetHexagon))
  (bind _hexagon_5 (Variables|Default|GetHexagon))
  (bind _hexagon_6 (Variables|Default|GetHexagon))
  (Utilities|Casting|CastToThirdPersonCharacter OtherActor)
  (Variables|Default|SetShoveBottomRight false)
  (Utilities|FlowControl|DoOnce false) ; enters at Reset
)

(event OnComponentBeginOverlap(BoxDown)
  (params (OverlappedComponent :type Primitive%20Component%20Object%20Reference) (OtherActor :type Actor%20Object%20Reference) (OtherComp :type Primitive%20Component%20Object%20Reference) (OtherBodyIndex :type Integer) (bFromSweep :type Boolean) (SweepResult :type Hit%20Result%20Structure%20%28by%20ref%29))
  (Utilities|Casting|CastToThirdPersonCharacter OtherActor)
  (Variables|Default|SetShoveDown true))

(event OnComponentEndOverlap(BoxDown)
  (params (OverlappedComponent :type Primitive%20Component%20Object%20Reference) (OtherActor :type Actor%20Object%20Reference) (OtherComp :type Primitive%20Component%20Object%20Reference) (OtherBodyIndex :type Integer))
  (bind _hexagon (Variables|Default|GetHexagon))
  (bind _hexagon_2 (Variables|Default|GetHexagon))
  (bind _hexagon_3 (Variables|Default|GetHexagon))
  (bind _hexagon_4 (Variables|Default|GetHexagon))
  (bind _hexagon_5 (Variables|Default|GetHexagon))
  (bind _hexagon_6 (Variables|Default|GetHexagon))
  (Utilities|Casting|CastToThirdPersonCharacter OtherActor)
  (Variables|Default|SetShoveDown false)
  (Utilities|FlowControl|DoOnce false) ; enters at Reset
)

(event OnComponentBeginOverlap(BoxTopLeft)
  (params (OverlappedComponent :type Primitive%20Component%20Object%20Reference) (OtherActor :type Actor%20Object%20Reference) (OtherComp :type Primitive%20Component%20Object%20Reference) (OtherBodyIndex :type Integer) (bFromSweep :type Boolean) (SweepResult :type Hit%20Result%20Structure%20%28by%20ref%29))
  (Utilities|Casting|CastToThirdPersonCharacter OtherActor)
  (Variables|Default|SetShoveTopLeft true))

(event OnComponentEndOverlap(BoxTopLeft)
  (params (OverlappedComponent :type Primitive%20Component%20Object%20Reference) (OtherActor :type Actor%20Object%20Reference) (OtherComp :type Primitive%20Component%20Object%20Reference) (OtherBodyIndex :type Integer))
  (bind _hexagon (Variables|Default|GetHexagon))
  (bind _hexagon_2 (Variables|Default|GetHexagon))
  (bind _hexagon_3 (Variables|Default|GetHexagon))
  (bind _hexagon_4 (Variables|Default|GetHexagon))
  (bind _hexagon_5 (Variables|Default|GetHexagon))
  (bind _hexagon_6 (Variables|Default|GetHexagon))
  (Utilities|Casting|CastToThirdPersonCharacter OtherActor)
  (Variables|Default|SetShoveTopLeft false)
  (Utilities|FlowControl|DoOnce false) ; enters at Reset
)

(event Custom|CustomEvent_1
  (Variables|Default|SetStartLocation (Transformation|GetActorTransform)))

(event Custom|CustomEvent
  (params (DeltaSeconds :type Float%20%28single-precision%29))
  (bind _hexagon (Variables|Default|GetHexagon))
  (bind _hexagon_2 (Variables|Default|GetHexagon))
  (bind _hexagon_3 (Variables|Default|GetHexagon))
  (bind _hexagon_4 (Variables|Default|GetHexagon))
  (bind _hexagon_5 (Variables|Default|GetHexagon))
  (bind _hexagon_6 (Variables|Default|GetHexagon))
  (if (Game|Player|IsInputKeyDown (Game|GetPlayerController 0) "R")
    (Transformation|SetActorTransform (Variables|Default|GetStartLocation) false true)
    (elif true
      (Utilities|FlowControl|DoOnce false
        (:Completed
          (Utilities|FlowControl|Sequence
            (:then_0
              (if (Variables|Default|GetShoveTopRight)
                (if (not (Variables|Default|GetBottomLeftBlocked))
                  (Physics|SetSimulatePhysics _hexagon_5 true)
                  (Physics|AddForce _hexagon_5 "20000.000000,-12000.000000, 0" "None" true)
                  (Utilities|FlowControl|Delay 0.5)
                  (Physics|SetSimulatePhysics _hexagon_5 false))))
            (:then_1
              (if (Variables|Default|GetShoveUp)
                (if (not (Variables|Default|GetDownBlocked))
                  (Physics|SetSimulatePhysics _hexagon true)
                  (Physics|AddForce _hexagon "0.000000,-32000.000000, 0" "None" true)
                  (Utilities|FlowControl|Delay 0.5)
                  (Physics|SetSimulatePhysics _hexagon false))))
            (:then_2
              (if (Variables|Default|GetShoveBottomRight)
                (if (not (Variables|Default|GetTopLeftBlocked))
                  (Physics|SetSimulatePhysics _hexagon_4 true)
                  (Physics|AddForce _hexagon_4 "20000.000000,12000.000000,0.000000" "None" true)
                  (Utilities|FlowControl|Delay 0.5)
                  (Physics|SetSimulatePhysics _hexagon_4 false))))
            (:then_3
              (if (Variables|Default|GetShoveDown)
                (if (not (Variables|Default|GetUpBlocked))
                  (Physics|SetSimulatePhysics _hexagon_2 true)
                  (Physics|AddForce _hexagon_2 "0.000000,32000.000000, 0" "None" true)
                  (Utilities|FlowControl|Delay 0.5)
                  (Physics|SetSimulatePhysics _hexagon_2 false))))
            (:then_4
              (if (Variables|Default|GetShoveBottomLeft)
                (if (not (Variables|Default|GetTopRightBlocked))
                  (Physics|SetSimulatePhysics _hexagon_3 true)
                  (Physics|AddForce _hexagon_3 "-20000.000000,12000.000000, 0" "None" true)
                  (Utilities|FlowControl|Delay 0.5)
                  (Physics|SetSimulatePhysics _hexagon_3 false))))
            (:then_5
              (if (Variables|Default|GetShoveTopLeft)
                (if (not (Variables|Default|GetBottomRightBlocked))
                  (Physics|SetSimulatePhysics _hexagon_6 true)
                  (Physics|AddForce _hexagon_6 "-20000.000000,-12000.000000, 0" "None" true)
                  (Utilities|FlowControl|Delay 0.5)
                  (Physics|SetSimulatePhysics _hexagon_6 false))))))))))

(fn ConstructionScript)