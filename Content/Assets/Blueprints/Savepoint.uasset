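; Savepoint actor that records a location and clears puzzle actors while the C key is held.
; Tick stores the player controller's own location, not the pawn's, in a variable and destroys every actor tagged "Puzzle".
; Three seconds after BeginPlay it opens ThirdPersonExampleMap, then sets the controller's location to that variable.
; The location lives only in this actor's variable, with no SaveGame or other persistence.
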(event EventBeginPlay
  (Utilities|FlowControl|Delay 3.0)
  (Game|OpenLevel(byName) "ThirdPersonExampleMap")
  (Transformation|SetActorLocation (Game|GetPlayerController 0) (Variables|Default|GetNewVar_1) false false))

(event Collision|EventActorBeginOverlap
  (params (OtherActor :type Actor%20Object%20Reference)))

(event EventTick
  (params (DeltaSeconds :type Float%20%28single-precision%29))
  (bind _returnvalue (Game|GetPlayerController 0))
  (if (Game|Player|IsInputKeyDown _returnvalue "C")
    (Variables|Default|SetNewVar_1 (Transformation|GetActorLocation _returnvalue))
    (bind _outactors (Actor|GetAllActorswithTag "Puzzle"))
    (for _array_element _outactors
      (Actor|DestroyActor _array_element))))

(fn ConstructionScript)