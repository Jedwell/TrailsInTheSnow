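; Pushable hexagonal block that the third-person character shoves in one of six directions with F.
; Side trigger boxes flag where the character stands, while check boxes block moves into occupied sides.
; A DoOnce-gated sequence plays an ice sound and a per-direction Timeline that slides the hexagon by delta time.
; Overlapping a DeletePhysics actor below flags a drop, which breaks the physics constraint and briefly simulates physics after a shove.
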(event OnComponentBeginOverlap(BoxTopRight)
  (params (OverlappedComponent :type Primitive%20Component%20Object%20Reference) (OtherActor :type Actor%20Object%20Reference) (OtherComp :type Primitive%20Component%20Object%20Reference) (OtherBodyIndex :type Integer) (bFromSweep :type Boolean) (SweepResult :type Hit%20Result%20Structure%20%28by%20ref%29))
  (Utilities|Casting|CastToThirdPersonCharacter OtherActor)
  (Variables|Default|SetShoveTopRight true))

(event OnComponentBeginOverlap(BoxUp)
  (params (OverlappedComponent :type Primitive%20Component%20Object%20Reference) (OtherActor :type Actor%20Object%20Reference) (OtherComp :type Primitive%20Component%20Object%20Reference) (OtherBodyIndex :type Integer) (bFromSweep :type Boolean) (SweepResult :type Hit%20Result%20Structure%20%28by%20ref%29))
  (Utilities|Casting|CastToThirdPersonCharacter OtherActor)
  (Variables|Default|SetShoveUp true))

(event OnComponentBeginOverlap(BoxBottomLeft)
  (params (OverlappedComponent :type Primitive%20Component%20Object%20Reference) (OtherActor :type Actor%20Object%20Reference) (OtherComp :type Primitive%20Component%20Object%20Reference) (OtherBodyIndex :type Integer) (bFromSweep :type Boolean) (SweepResult :type Hit%20Result%20Structure%20%28by%20ref%29))
  (Utilities|Casting|CastToThirdPersonCharacter OtherActor)
  (Variables|Default|SetShoveBottomLeft true))

(event OnComponentEndOverlap(BoxBottomLeft)
  (params (OverlappedComponent :type Primitive%20Component%20Object%20Reference) (OtherActor :type Actor%20Object%20Reference) (OtherComp :type Primitive%20Component%20Object%20Reference) (OtherBodyIndex :type Integer))
  (Utilities|Casting|CastToThirdPersonCharacter OtherActor)
  (Variables|Default|SetShoveBottomLeft false))

(event OnComponentBeginOverlap(BoxCheckTopRight)
  (params (OverlappedComponent :type Primitive%20Component%20Object%20Reference) (OtherActor :type Actor%20Object%20Reference) (OtherComp :type Primitive%20Component%20Object%20Reference) (OtherBodyIndex :type Integer) (bFromSweep :type Boolean) (SweepResult :type Hit%20Result%20Structure%20%28by%20ref%29))
  (Utilities|Casting|CastToThirdPersonCharacter OtherActor
    (:CastFailed
      (Variables|Default|SetTopRightBlocked true))))

(event OnComponentEndOverlap(BoxCheckTopRight)
  (params (OverlappedComponent :type Primitive%20Component%20Object%20Reference) (OtherActor :type Actor%20Object%20Reference) (OtherComp :type Primitive%20Component%20Object%20Reference) (OtherBodyIndex :type Integer))
  (Utilities|Casting|CastToThirdPersonCharacter OtherActor
    (:CastFailed
      (Variables|Default|SetTopRightBlocked false))))

(event OnComponentBeginOverlap(BoxCheckUp)
  (params (OverlappedComponent :type Primitive%20Component%20Object%20Reference) (OtherActor :type Actor%20Object%20Reference) (OtherComp :type Primitive%20Component%20Object%20Reference) (OtherBodyIndex :type Integer) (bFromSweep :type Boolean) (SweepResult :type Hit%20Result%20Structure%20%28by%20ref%29))
  (Utilities|Casting|CastToThirdPersonCharacter OtherActor
    (:CastFailed
      (Variables|Default|SetUpBlocked true))))

(event OnComponentEndOverlap(BoxCheckUp)
  (params (OverlappedComponent :type Primitive%20Component%20Object%20Reference) (OtherActor :type Actor%20Object%20Reference) (OtherComp :type Primitive%20Component%20Object%20Reference) (OtherBodyIndex :type Integer))
  (Utilities|Casting|CastToThirdPersonCharacter OtherActor
    (:CastFailed
      (Variables|Default|SetUpBlocked false))))

(event OnComponentBeginOverlap(BoxCheckDown)
  (params (OverlappedComponent :type Primitive%20Component%20Object%20Reference) (OtherActor :type Actor%20Object%20Reference) (OtherComp :type Primitive%20Component%20Object%20Reference) (OtherBodyIndex :type Integer) (bFromSweep :type Boolean) (SweepResult :type Hit%20Result%20Structure%20%28by%20ref%29))
  (Utilities|Casting|CastToThirdPersonCharacter OtherActor
    (:CastFailed
      (Variables|Default|SetDownBlocked true))))

(event OnComponentEndOverlap(BoxCheckDown)
  (params (OverlappedComponent :type Primitive%20Component%20Object%20Reference) (OtherActor :type Actor%20Object%20Reference) (OtherComp :type Primitive%20Component%20Object%20Reference) (OtherBodyIndex :type Integer))
  (Utilities|Casting|CastToThirdPersonCharacter OtherActor
    (:CastFailed
      (Variables|Default|SetDownBlocked false))))

(event OnComponentBeginOverlap(BoxCheckTopLeft)
  (params (OverlappedComponent :type Primitive%20Component%20Object%20Reference) (OtherActor :type Actor%20Object%20Reference) (OtherComp :type Primitive%20Component%20Object%20Reference) (OtherBodyIndex :type Integer) (bFromSweep :type Boolean) (SweepResult :type Hit%20Result%20Structure%20%28by%20ref%29))
  (Utilities|Casting|CastToThirdPersonCharacter OtherActor
    (:CastFailed
      (Variables|Default|SetTopLeftBlocked true))))

(event OnComponentEndOverlap(BoxCheckTopLeft)
  (params (OverlappedComponent :type Primitive%20Component%20Object%20Reference) (OtherActor :type Actor%20Object%20Reference) (OtherComp :type Primitive%20Component%20Object%20Reference) (OtherBodyIndex :type Integer))
  (Utilities|Casting|CastToThirdPersonCharacter OtherActor
    (:CastFailed
      (Variables|Default|SetTopLeftBlocked false))))

(event OnComponentEndOverlap(BoxTopRight)
  (params (OverlappedComponent :type Primitive%20Component%20Object%20Reference) (OtherActor :type Actor%20Object%20Reference) (OtherComp :type Primitive%20Component%20Object%20Reference) (OtherBodyIndex :type Integer))
  (Utilities|Casting|CastToThirdPersonCharacter OtherActor)
  (Variables|Default|SetShoveTopRight false))

(event OnComponentBeginOverlap(BoxCheckBottomLeft)
  (params (OverlappedComponent :type Primitive%20Component%20Object%20Reference) (OtherActor :type Actor%20Object%20Reference) (OtherComp :type Primitive%20Component%20Object%20Reference) (OtherBodyIndex :type Integer) (bFromSweep :type Boolean) (SweepResult :type Hit%20Result%20Structure%20%28by%20ref%29))
  (Utilities|Casting|CastToThirdPersonCharacter OtherActor
    (:CastFailed
      (Variables|Default|SetBottomLeftBlocked true))))

(event OnComponentEndOverlap(BoxCheckBottomLeft)
  (params (OverlappedComponent :type Primitive%20Component%20Object%20Reference) (OtherActor :type Actor%20Object%20Reference) (OtherComp :type Primitive%20Component%20Object%20Reference) (OtherBodyIndex :type Integer))
  (Utilities|Casting|CastToThirdPersonCharacter OtherActor
    (:CastFailed
      (Variables|Default|SetBottomLeftBlocked false))))

(event OnComponentBeginOverlap(BoxCheckBottomRight)
  (params (OverlappedComponent :type Primitive%20Component%20Object%20Reference) (OtherActor :type Actor%20Object%20Reference) (OtherComp :type Primitive%20Component%20Object%20Reference) (OtherBodyIndex :type Integer) (bFromSweep :type Boolean) (SweepResult :type Hit%20Result%20Structure%20%28by%20ref%29))
  (Utilities|Casting|CastToThirdPersonCharacter OtherActor
    (:CastFailed
      (Variables|Default|SetBottomRightBlocked true))))

(event OnComponentEndOverlap(BoxCheckBottomRight)
  (params (OverlappedComponent :type Primitive%20Component%20Object%20Reference) (OtherActor :type Actor%20Object%20Reference) (OtherComp :type Primitive%20Component%20Object%20Reference) (OtherBodyIndex :type Integer))
  (Utilities|Casting|CastToThirdPersonCharacter OtherActor
    (:CastFailed
      (Variables|Default|SetBottomRightBlocked false))))

(event OnComponentBeginOverlap(Below)
  (params (OverlappedComponent :type Primitive%20Component%20Object%20Reference) (OtherActor :type Actor%20Object%20Reference) (OtherComp :type Primitive%20Component%20Object%20Reference) (OtherBodyIndex :type Integer) (bFromSweep :type Boolean) (SweepResult :type Hit%20Result%20Structure%20%28by%20ref%29))
  (Utilities|Casting|CastToDeletePhysics OtherActor)
  (Variables|Default|SetDrop true))

(event OnComponentEndOverlap(BoxUp)
  (params (OverlappedComponent :type Primitive%20Component%20Object%20Reference) (OtherActor :type Actor%20Object%20Reference) (OtherComp :type Primitive%20Component%20Object%20Reference) (OtherBodyIndex :type Integer))
  (Utilities|Casting|CastToThirdPersonCharacter OtherActor)
  (Variables|Default|SetShoveUp false))

(event OnComponentBeginOverlap(BoxBottomRight)
  (params (OverlappedComponent :type Primitive%20Component%20Object%20Reference) (OtherActor :type Actor%20Object%20Reference) (OtherComp :type Primitive%20Component%20Object%20Reference) (OtherBodyIndex :type Integer) (bFromSweep :type Boolean) (SweepResult :type Hit%20Result%20Structure%20%28by%20ref%29))
  (Utilities|Casting|CastToThirdPersonCharacter OtherActor)
  (Variables|Default|SetShoveBottomRight true))

(event OnComponentEndOverlap(BoxBottomRight)
  (params (OverlappedComponent :type Primitive%20Component%20Object%20Reference) (OtherActor :type Actor%20Object%20Reference) (OtherComp :type Primitive%20Component%20Object%20Reference) (OtherBodyIndex :type Integer))
  (Utilities|Casting|CastToThirdPersonCharacter OtherActor)
  (Variables|Default|SetShoveBottomRight false))

(event OnComponentBeginOverlap(BoxDown)
  (params (OverlappedComponent :type Primitive%20Component%20Object%20Reference) (OtherActor :type Actor%20Object%20Reference) (OtherComp :type Primitive%20Component%20Object%20Reference) (OtherBodyIndex :type Integer) (bFromSweep :type Boolean) (SweepResult :type Hit%20Result%20Structure%20%28by%20ref%29))
  (Utilities|Casting|CastToThirdPersonCharacter OtherActor)
  (Variables|Default|SetShoveDown true))

(event OnComponentEndOverlap(BoxDown)
  (params (OverlappedComponent :type Primitive%20Component%20Object%20Reference) (OtherActor :type Actor%20Object%20Reference) (OtherComp :type Primitive%20Component%20Object%20Reference) (OtherBodyIndex :type Integer))
  (Utilities|Casting|CastToThirdPersonCharacter OtherActor)
  (Variables|Default|SetShoveDown false))

(event OnComponentBeginOverlap(BoxTopLeft)
  (params (OverlappedComponent :type Primitive%20Component%20Object%20Reference) (OtherActor :type Actor%20Object%20Reference) (OtherComp :type Primitive%20Component%20Object%20Reference) (OtherBodyIndex :type Integer) (bFromSweep :type Boolean) (SweepResult :type Hit%20Result%20Structure%20%28by%20ref%29))
  (Utilities|Casting|CastToThirdPersonCharacter OtherActor)
  (Variables|Default|SetShoveTopLeft true))

(event OnComponentEndOverlap(BoxTopLeft)
  (params (OverlappedComponent :type Primitive%20Component%20Object%20Reference) (OtherActor :type Actor%20Object%20Reference) (OtherComp :type Primitive%20Component%20Object%20Reference) (OtherBodyIndex :type Integer))
  (Utilities|Casting|CastToThirdPersonCharacter OtherActor)
  (Variables|Default|SetShoveTopLeft false))

(event EventTick
  (params (DeltaSeconds :type Float%20%28single-precision%29))
  (bind _hexagon (Variables|Default|GetHexagon))
  (bind _hexagon_2 (Variables|Default|GetHexagon))
  (bind _hexagon_3 (Variables|Default|GetHexagon))
  (bind _hexagon_4 (Variables|Default|GetHexagon))
  (bind _hexagon_5 (Variables|Default|GetHexagon))
  (bind _hexagon_6 (Variables|Default|GetHexagon))
  (Variables|Default|SetDeltaTime DeltaSeconds)
  (if (Game|Player|WasInputKeyJustPressed (Game|GetPlayerController 0) "F")
    (Utilities|FlowControl|Delay 0.35)
    (Utilities|FlowControl|DoOnce false :!label _label
      (:Completed
        (Utilities|FlowControl|Sequence
          (:then_0
            (if (Variables|Default|GetShoveTopRight)
              (if (not (and (Variables|Default|GetBottomLeftBlocked) (not (Variables|Default|GetShoving))))
                (Audio|PlaySoundatLocation "/Game/Sounds/Footsteps/sfx_footsteps_ice_01.sfx_footsteps_ice_01" "0, 0, 0" "0, 0, 0" 1.0 1.0 0.0 0 0 0)
                (Variables|Default|SetShoving true)
                (Timeline|Timeline_0 PlayFromStart
                  (:Update
                    (Class|SceneComponent|AddLocalTransform _hexagon_2 (Math|Transform|MakeTransform (* "129.199997,-75.500000,0.000000" (Variables|Default|GetDeltaTime)) "0, 0, 0" (Variables|/Script/Engine.SceneComponent|GetRelativeScale3D _hexagon_2)) false false))
                  (:Finished
                    (Variables|Default|SetShoving false :!label _label_2)
                    (if (Variables|Default|GetDrop)
                      (Utilities|FlowControl|Delay 0.5)
                      (Components|DestroyComponent (Variables|Default|GetPhysicsConstraint))
                      (Physics|SetSimulatePhysics (Variables|Default|GetHexagon) true)
                      (Utilities|FlowControl|Delay 2.0)
                      (Physics|SetSimulatePhysics (Variables|Default|GetHexagon) false)
                      (else
                        (goto _label Reset))))))
              (else
                (Utilities|FlowControl|Delay 0.5 :!label _label_3)
                (goto _label Reset))))
          (:then_1
            (if (Variables|Default|GetShoveUp)
              (if (not (and (Variables|Default|GetDownBlocked) (not (Variables|Default|GetShoving))))
                (Audio|PlaySoundatLocation "/Game/Sounds/Footsteps/sfx_footsteps_ice_01.sfx_footsteps_ice_01" "0, 0, 0" "0, 0, 0" 1.0 1.0 0.0 0 0 0)
                (Variables|Default|SetShoving true)
                (Timeline|Timeline_1 PlayFromStart
                  (:Update
                    (Class|SceneComponent|AddLocalTransform _hexagon_3 (Math|Transform|MakeTransform (* "0,-150.500000, 0" (Variables|Default|GetDeltaTime)) "0, 0, 0" (Variables|/Script/Engine.SceneComponent|GetRelativeScale3D _hexagon_3)) false false))
                  (:Finished
                    (goto _label_2))))
              (else
                (goto _label_3))))
          (:then_2
            (if (Variables|Default|GetShoveBottomRight)
              (if (not (and (Variables|Default|GetTopLeftBlocked) (not (Variables|Default|GetShoving))))
                (Audio|PlaySoundatLocation "/Game/Sounds/Footsteps/sfx_footsteps_ice_01.sfx_footsteps_ice_01" "0, 0, 0" "0, 0, 0" 1.0 1.0 0.0 0 0 0)
                (Variables|Default|SetShoving true)
                (Timeline|Timeline_2 PlayFromStart
                  (:Update
                    (Class|SceneComponent|AddLocalTransform _hexagon_4 (Math|Transform|MakeTransform (* "129.199997,75.500000, 0" (Variables|Default|GetDeltaTime)) "0, 0, 0" (Variables|/Script/Engine.SceneComponent|GetRelativeScale3D _hexagon_4)) false false)
                    (goto _label_2))))
              (else
                (goto _label_3))))
          (:then_3
            (if (Variables|Default|GetShoveDown)
              (if (not (and (Variables|Default|GetUpBlocked) (not (Variables|Default|GetShoving))))
                (Audio|PlaySoundatLocation "/Game/Sounds/Footsteps/sfx_footsteps_ice_01.sfx_footsteps_ice_01" "0, 0, 0" "0, 0, 0" 1.0 1.0 0.0 0 0 0)
                (Variables|Default|SetShoving true)
                (Timeline|Timeline_3 PlayFromStart
                  (:Update
                    (Class|SceneComponent|AddLocalTransform _hexagon_5 (Math|Transform|MakeTransform (* "0,150.500000, 0" (Variables|Default|GetDeltaTime)) "0, 0, 0" (Variables|/Script/Engine.SceneComponent|GetRelativeScale3D _hexagon_5)) false false)
                    (goto _label_2))))
              (else
                (goto _label_3))))
          (:then_4
            (if (Variables|Default|GetShoveBottomLeft)
              (if (not (and (Variables|Default|GetTopRightBlocked) (not (Variables|Default|GetShoving))))
                (Audio|PlaySoundatLocation "/Game/Sounds/Footsteps/sfx_footsteps_ice_01.sfx_footsteps_ice_01" "0, 0, 0" "0, 0, 0" 1.0 1.0 0.0 0 0 0)
                (Variables|Default|SetShoving true)
                (Timeline|Timeline_4 PlayFromStart
                  (:Update
                    (Class|SceneComponent|AddLocalTransform _hexagon_6 (Math|Transform|MakeTransform (* "-129.199997,75.500000, 0" (Variables|Default|GetDeltaTime)) "0, 0, 0" (Variables|/Script/Engine.SceneComponent|GetRelativeScale3D _hexagon_6)) false false)
                    (goto _label_2))))
              (else
                (goto _label_3))))
          (:then_5
            (if (Variables|Default|GetShoveTopLeft)
              (if (not (and (Variables|Default|GetBottomRightBlocked) (not (Variables|Default|GetShoving))))
                (Audio|PlaySoundatLocation "/Game/Sounds/Footsteps/sfx_footsteps_ice_01.sfx_footsteps_ice_01" "0, 0, 0" "0, 0, 0" 1.0 1.0 0.0 0 0 0)
                (Variables|Default|SetShoving true)
                (Timeline|Timeline_5 PlayFromStart
                  (:Update
                    (Class|SceneComponent|AddLocalTransform _hexagon (Math|Transform|MakeTransform (* "-129.199997,-75.500000, 0" (Variables|Default|GetDeltaTime)) "0, 0, 0" (Variables|/Script/Engine.SceneComponent|GetRelativeScale3D _hexagon)) false false)
                    (goto _label_2))))
              (else
                (goto _label_3)))))))))

(fn ConstructionScript)