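; Final runestone of a musical statue riddle, which plays a flute note when the player presses F inside its interaction box.
; Tick polls the key behind a cooldown, then checks the character's Statue4Interacted flag.
; If set, it lights up, plays the crystal sequence, removes crystals with effects and camera fades, then starts self-restarting level music.
; Otherwise it clears the first three statue flags and dims Runestones 1–3.
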(event OnComponentBeginOverlap(InteractionBox)
  (params (OverlappedComponent :type Primitive%20Component%20Object%20Reference) (OtherActor :type Actor%20Object%20Reference) (OtherComp :type Primitive%20Component%20Object%20Reference) (OtherBodyIndex :type Integer) (bFromSweep :type Boolean) (SweepResult :type Hit%20Result%20Structure%20%28by%20ref%29))
  (bind _asthird_person_character (Utilities|Casting|CastToThirdPersonCharacter OtherActor))
  (Variables|Default|SetPlayerOverlap true))

(event OnComponentEndOverlap(InteractionBox)
  (params (OverlappedComponent :type Primitive%20Component%20Object%20Reference) (OtherActor :type Actor%20Object%20Reference) (OtherComp :type Primitive%20Component%20Object%20Reference) (OtherBodyIndex :type Integer))
  (Utilities|Casting|CastToThirdPersonCharacter OtherActor)
  (Variables|Default|SetPlayerOverlap false))

(event Custom|OnAudioFinished_Event_0
  (bind _returnvalue (Audio|SpawnSoundAttached "/Game/Assets/SFX/Trails_In_The_Snow_Level_PreMaster.Trails_In_The_Snow_Level_PreMaster" (Variables|/Script/Engine.Character|GetMesh (Game|GetPlayerCharacter 0)) "None" "0, 0, 0" "0, 0, 0" "KeepRelativeOffset" false 1.0 1.0 0.0 0 0 false))
  (EventDispatchers|AssignOnAudioFinished _returnvalue (delegate Custom|OnAudioFinished_Event_0)))

(event EventBeginPlay
  (Components|Activation|SetActive (Variables|Default|GetRunestoneGlow) false false)
  (bind _newtrack_0 (Timeline|Timeline_0 Play)
    (:Update
      (Class|SceneComponent|AddLocalTransform (Variables|Default|GetSphere) (Math|Transform|MakeTransform _newtrack_0 "0, 0, 0" "1,1,1") false false))))

(event EventTick
  (params (DeltaSeconds :type Float%20%28single-precision%29))
  (bind _returnvalue (Game|GetPlayerController 0))
  (bind _playercameramanager (Variables|/Script/Engine.PlayerController|GetPlayerCameraManager _returnvalue))
  (if (Variables|Default|GetPlayerOverlap)
    (if (Game|Player|WasInputKeyJustPressed (Game|GetPlayerController 0) "F")
      (Utilities|FlowControl|Delay 0.35)
      (Utilities|FlowControl|DoOnce false :!label _label
        (:Completed
          (Utilities|FlowControl|Sequence
            (:then_0
              (Audio|PlaySoundatLocation "/Game/Assets/SFX/sfx_musicriddle_05_flute.sfx_musicriddle_05_flute" (Transformation|GetActorLocation) "0, 0, 0" 1.0 1.0 0.0 0 0 0)
              (if (Variables|/Game/ThirdPersonBP/Blueprints/ThirdPersonCharacter.ThirdPersonCharacter_C|GetStatue4Interacted (stale OnComponentBeginOverlap(InteractionBox) _asthird_person_character))
                (Utilities|FlowControl|DoOnce false
                  (:Completed
                    (Components|Activation|SetActive (Variables|Default|GetRunestoneGlow) true true)
                    (Rendering|Material|SetMaterial (Variables|Debug|GetStaticMeshComponent) 0 "/Game/Geometry/Textures/Runestone5/Runestone5.Runestone5")
                    (Rendering|Material|SetMaterial (Variables|Default|GetSphere) 0 "/Game/Geometry/Textures/Runestone5/Runestone5.Runestone5")
                    (Utilities|FlowControl|Delay 1.0)
                    (bind _returnvalue_2 (Sequencer|Player|CreateLevelSequencePlayer "/Game/Assets/Rigs/CrystalRig.CrystalRig"))
                    (Sequencer|Player|Play _returnvalue_2 :!class /Script/MovieScene.MovieSceneSequencePlayer)
                    (bind _outactors (Actor|GetAllActorsOfClass "/Game/Assets/Blueprints/Kristall_Blueprint.Kristall_Blueprint_C"))
                    (for _array_element _outactors
                      (Utilities|FlowControl|Delay 4.0)
                      (AddComponent|AddNiagaraComponent _array_element false)
                      (Rendering|SetVisibility (Variables|/Script/Engine.Actor|GetRootComponent _array_element) false false)
                      (Audio|PlaySoundatLocation "/Game/Assets/SFX/sfx_musicriddle_finished.sfx_musicriddle_finished" "0, 0, 0" "0, 0, 0" 1.0 1.0 0.0 0 0 0)
                      (Utilities|FlowControl|Delay 2.0)
                      (Actor|DestroyActor _array_element)
                      (CameraFades|StartCameraFade :self _playercameramanager :ToAlpha 1.0 :Duration 1.0 :bHoldWhenFinished true)
                      (Utilities|FlowControl|Delay 0.95)
                      (CameraFades|StartCameraFade :self _playercameramanager :FromAlpha 1.0 :Duration 1.0 :bHoldWhenFinished true))
                    (Utilities|FlowControl|Delay 1.5)
                    (bind _returnvalue_3 (Audio|SpawnSoundAttached "/Game/Assets/SFX/Trails_In_The_Snow_Level_PreMaster.Trails_In_The_Snow_Level_PreMaster" (Variables|/Script/Engine.Character|GetMesh (Game|GetPlayerCharacter 0)) "None" "0, 0, 0" "0, 0, 0" "KeepRelativeOffset" false 1.0 1.0 0.0 0 0 false))
                    (EventDispatchers|AssignOnAudioFinished _returnvalue_3 (delegate Custom|OnAudioFinished_Event_0))))
                (else
                  (Variables|/Game/ThirdPersonBP/Blueprints/ThirdPersonCharacter.ThirdPersonCharacter_C|SetStatue1Interacted (stale OnComponentBeginOverlap(InteractionBox) _asthird_person_character) false)
                  (Variables|/Game/ThirdPersonBP/Blueprints/ThirdPersonCharacter.ThirdPersonCharacter_C|SetStatue2Interacted (stale OnComponentBeginOverlap(InteractionBox) _asthird_person_character) false)
                  (Variables|/Game/ThirdPersonBP/Blueprints/ThirdPersonCharacter.ThirdPersonCharacter_C|SetStatue3Interacted (stale OnComponentBeginOverlap(InteractionBox) _asthird_person_character) false)
                  (Utilities|FlowControl|Sequence
                    (:then_0
                      (bind _outactors_2 (Actor|GetAllActorsOfClass "/Game/Assets/Blueprints/Runestone_1.Runestone_1_C"))
                      (for _array_element_2 _outactors_2
                        (Components|Activation|SetActive (Variables|/Game/Assets/Blueprints/Runestone_1.Runestone_1_C|GetRunestoneGlow _array_element_2) false false)
                        (Rendering|Material|SetMaterial (Variables|/Game/Assets/Blueprints/Runestone_1.Runestone_1_C|GetSphere _array_element_2) 0 "/Game/Geometry/Textures/Runestone1/Runestone1_NoEmissive.Runestone1_NoEmissive")
                        (Rendering|Material|SetMaterial (Variables|/Script/Engine.StaticMeshActor|GetStaticMeshComponent _array_element_2) 0 "/Game/Geometry/Textures/Runestone1/Runestone1_NoEmissive.Runestone1_NoEmissive")))
                    (:then_1
                      (bind _outactors_3 (Actor|GetAllActorsOfClass "/Game/Assets/Blueprints/Runestone_2.Runestone_2_C"))
                      (for _array_element_3 _outactors_3
                        (Components|Activation|SetActive (Variables|/Game/Assets/Blueprints/Runestone_2.Runestone_2_C|GetRunestoneGlow _array_element_3) false false)
                        (Rendering|Material|SetMaterial (Variables|/Game/Assets/Blueprints/Runestone_2.Runestone_2_C|GetSphere _array_element_3) 0 "/Game/Geometry/Textures/Runestone2/Runestone2_NoEmissive.Runestone2_NoEmissive")
                        (Rendering|Material|SetMaterial (Variables|/Script/Engine.StaticMeshActor|GetStaticMeshComponent _array_element_3) 0 "/Game/Geometry/Textures/Runestone2/Runestone2_NoEmissive.Runestone2_NoEmissive")))
                    (:then_2
                      (bind _outactors_4 (Actor|GetAllActorsOfClass "/Game/Assets/Blueprints/Runestone_3.Runestone_3_C"))
                      (for _array_element_4 _outactors_4
                        (Components|Activation|SetActive (Variables|/Game/Assets/Blueprints/Runestone_3.Runestone_3_C|GetRunestoneGlow _array_element_4) false false)
                        (Rendering|Material|SetMaterial (Variables|/Game/Assets/Blueprints/Runestone_3.Runestone_3_C|GetSphere _array_element_4) 0 "/Game/Geometry/Textures/Runestone3/Runestone3_NoEmissive.Runestone3_NoEmissive")
                        (Rendering|Material|SetMaterial (Variables|/Script/Engine.StaticMeshActor|GetStaticMeshComponent _array_element_4) 0 "/Game/Geometry/Textures/Runestone3/Runestone3_NoEmissive.Runestone3_NoEmissive")))))))
            (:then_1
              (Utilities|FlowControl|Delay 2.0)
              (goto _label Reset))))))))

(fn ConstructionScript)