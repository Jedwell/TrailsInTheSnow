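; Interactable statue, the fifth in an ordered interaction puzzle tracked by flags on ThirdPersonCharacter.
; An interaction box caches the overlapping character, and Tick polls the F key while they are inside.
; If the fourth statue's flag is set, it plays a bird sound once and destroys the player character.
; Otherwise it clears the first three statues' flags, resetting that progress.
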(event OnComponentBeginOverlap(InteractionBox)
  (params (OverlappedComponent :type Primitive%20Component%20Object%20Reference) (OtherActor :type Actor%20Object%20Reference) (OtherComp :type Primitive%20Component%20Object%20Reference) (OtherBodyIndex :type Integer) (bFromSweep :type Boolean) (SweepResult :type Hit%20Result%20Structure%20%28by%20ref%29))
  (bind _asthird_person_character (Utilities|Casting|CastToThirdPersonCharacter OtherActor))
  (Variables|Default|SetPlayerOverlap true))

(event OnComponentEndOverlap(InteractionBox)
  (params (OverlappedComponent :type Primitive%20Component%20Object%20Reference) (OtherActor :type Actor%20Object%20Reference) (OtherComp :type Primitive%20Component%20Object%20Reference) (OtherBodyIndex :type Integer))
  (Utilities|Casting|CastToThirdPersonCharacter OtherActor)
  (Variables|Default|SetPlayerOverlap false))

(event EventTick
  (params (DeltaSeconds :type Float%20%28single-precision%29))
  (if (Variables|Default|GetPlayerOverlap)
    (if (Game|Player|IsInputKeyDown (Game|GetPlayerController 0) "F")
      (if (Variables|/Game/ThirdPersonBP/Blueprints/ThirdPersonCharacter.ThirdPersonCharacter_C|GetStatue4Interacted (stale OnComponentBeginOverlap(InteractionBox) _asthird_person_character))
        (Utilities|FlowControl|DoOnce false
          (:Completed
            (Audio|PlaySoundatLocation "/Game/StarterContent/Audio/Starter_Birds01.Starter_Birds01" (Transformation|GetActorLocation) "0, 0, 0" 1.0 1.0 0.0 0 0 0)
            (Actor|DestroyActor (stale OnComponentBeginOverlap(InteractionBox) _asthird_person_character))))
        (else
          (Variables|/Game/ThirdPersonBP/Blueprints/ThirdPersonCharacter.ThirdPersonCharacter_C|SetStatue1Interacted (stale OnComponentBeginOverlap(InteractionBox) _asthird_person_character) false)
          (Variables|/Game/ThirdPersonBP/Blueprints/ThirdPersonCharacter.ThirdPersonCharacter_C|SetStatue2Interacted (stale OnComponentBeginOverlap(InteractionBox) _asthird_person_character) false)
          (Variables|/Game/ThirdPersonBP/Blueprints/ThirdPersonCharacter.ThirdPersonCharacter_C|SetStatue3Interacted (stale OnComponentBeginOverlap(InteractionBox) _asthird_person_character) false))))))

(fn ConstructionScript)