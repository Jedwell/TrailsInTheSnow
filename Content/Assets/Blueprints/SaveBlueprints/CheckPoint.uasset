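; Checkpoint actor that saves the player's respawn point and lets R return them there while resetting puzzle objects.
; BeginPlay records the locations of all actors tagged "Puzzle"; a player overlapping the trigger volume saves the checkpoint's location.
; The first overlap by any actor opens a Tick gate that polls R.
; While R is held, each tick teleports the player back, destroys tagged actors and spawns Kubus replacements at recorded locations.
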(event OnComponentBeginOverlap(TriggerVolume)
  (params (OverlappedComponent :type Primitive%20Component%20Object%20Reference) (OtherActor :type Actor%20Object%20Reference) (OtherComp :type Primitive%20Component%20Object%20Reference) (OtherBodyIndex :type Integer) (bFromSweep :type Boolean) (SweepResult :type Hit%20Result%20Structure%20%28by%20ref%29))
  (Utilities|FlowControl|Sequence
    (:then_0
      (Utilities|FlowControl|DoOnce false
        (:Completed
          (Utilities|FlowControl|Gate true) ; enters at Open
        )))
    (:then_1
      (if (Actor|ActorHasTag OtherActor "Player")
        (Variables|Default|SetPlayerSaveLocation (Transformation|GetActorLocation))
        (bind _asthird_person_character (Utilities|Casting|CastToThirdPersonCharacter OtherActor))
        (Variables|Default|SetPlayer _asthird_person_character)))))

(event EventBeginPlay
  (bind _outactors (Actor|GetAllActorswithTag "Puzzle"))
  (for _array_element _outactors
    (Utilities|Array|Add (Variables|Default|GetPuzzleLocations) (Transformation|GetActorLocation _array_element))))

(event Collision|EventActorBeginOverlap
  (params (OtherActor :type Actor%20Object%20Reference)))

(event EventTick
  (params (DeltaSeconds :type Float%20%28single-precision%29))
  (Utilities|FlowControl|Gate true
    (:Exit
      (if (Game|Player|IsInputKeyDown (Game|GetPlayerController 0) "R")
        (Transformation|SetActorLocation (Variables|Default|GetPlayer) (Variables|Default|GetPlayerSaveLocation) false true)
        (bind _outactors (Actor|GetAllActorswithTag "Puzzle"))
        (for (_array_element _array_index) _outactors
          (Actor|DestroyActor _array_element)
          (Game|SpawnActorfromClass "/Game/Assets/Blueprints/Kubus.Kubus_C" (Math|Transform|MakeTransform (Utilities|Array|Get(acopy) (Variables|Default|GetPuzzleLocations) _array_index) "0, 0, 0" "2.500000,2.500000,2.500000") "AlwaysSpawn" 0 0))))))

(fn ConstructionScript)