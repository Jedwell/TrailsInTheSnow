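; Second runestone in an ordered, musical interaction puzzle, activated by pressing F inside its interaction box.
; Overlap stores the player character and enables a key check on Tick, which plays a piano sound after a short delay, throttled by a resetting DoOnce.
; If Statue1Interacted is set on the character, the first press also sets Statue2Interacted, activates the glow and swaps materials.
; A timeline started on BeginPlay moves the sphere.
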(event OnComponentBeginOverlap(InteractionBox)
  (params (OverlappedComponent :type Primitive%20Component%20Object%20Reference) (OtherActor :type Actor%20Object%20Reference) (OtherComp :type Primitive%20Component%20Object%20Reference) (OtherBodyIndex :type Integer) (bFromSweep :type Boolean) (SweepResult :type Hit%20Result%20Structure%20%28by%20ref%29))
  (bind _asthird_person_character (Utilities|Casting|CastToThirdPersonCharacter OtherActor))
  (Variables|Default|SetPlayerOverlap true))

(event OnComponentEndOverlap(InteractionBox)
  (params (OverlappedComponent :type Primitive%20Component%20Object%20Reference) (OtherActor :type Actor%20Object%20Reference) (OtherComp :type Primitive%20Component%20Object%20Reference) (OtherBodyIndex :type Integer))
  (Utilities|Casting|CastToThirdPersonCharacter OtherActor)
  (Variables|Default|SetPlayerOverlap false))

(event EventBeginPlay
  (Components|Activation|SetActive (Variables|Default|GetRunestoneGlow) false false)
  (bind _newtrack_0 (Timeline|Timeline_0 Play)
    (:Update
      (Class|SceneComponent|AddLocalTransform (Variables|Default|GetSphere) (Math|Transform|MakeTransform _newtrack_0 "0, 0, 0" "1,1,1") false false))))

(event EventTick
  (params (DeltaSeconds :type Float%20%28single-precision%29))
  (if (Variables|Default|GetPlayerOverlap)
    (if (Game|Player|WasInputKeyJustPressed (Game|GetPlayerController 0) "F")
      (Utilities|FlowControl|Delay 0.35)
      (Utilities|FlowControl|DoOnce false :!label _label
        (:Completed
          (Utilities|FlowControl|Sequence
            (:then_0
              (Audio|PlaySoundatLocation "/Game/Assets/SFX/sfx_musicriddle_02_piano.sfx_musicriddle_02_piano" (Transformation|GetActorLocation) "0, 0, 0" 1.0 1.0 0.0 0 0 0)
              (if (Variables|/Game/ThirdPersonBP/Blueprints/ThirdPersonCharacter.ThirdPersonCharacter_C|GetStatue1Interacted (stale OnComponentBeginOverlap(InteractionBox) _asthird_person_character))
                (if (not (Variables|/Game/ThirdPersonBP/Blueprints/ThirdPersonCharacter.ThirdPersonCharacter_C|GetStatue2Interacted (stale OnComponentBeginOverlap(InteractionBox) _asthird_person_character)))
                  (Variables|/Game/ThirdPersonBP/Blueprints/ThirdPersonCharacter.ThirdPersonCharacter_C|SetStatue2Interacted (stale OnComponentBeginOverlap(InteractionBox) _asthird_person_character) true)
                  (Components|Activation|SetActive (Variables|Default|GetRunestoneGlow) true true)
                  (Rendering|Material|SetMaterial (Variables|Debug|GetStaticMeshComponent) 0 "/Game/Geometry/Textures/Runestone2/Runestone2.Runestone2")
                  (Rendering|Material|SetMaterial (Variables|Default|GetSphere) 0 "/Game/Geometry/Textures/Runestone2/Runestone2.Runestone2"))))
            (:then_1
              (Utilities|FlowControl|Delay 2.0)
              (goto _label Reset))))))))

(fn ConstructionScript)