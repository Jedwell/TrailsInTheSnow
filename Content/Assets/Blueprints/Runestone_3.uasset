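; Third runestone in an ordered interaction puzzle, activated by holding F while the ThirdPersonCharacter overlaps its InteractionBox.
; Tick polls the key: if Statue2Interacted is set, it plays an explosion sound every frame F is held, sets Statue3Interacted and lights RunestoneGlow.
; Otherwise it clears only Statue1Interacted and switches off the glow on all Runestone_1 to 5 actors.
; BeginPlay disables the glow and starts a timeline that offsets the Sphere.
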(event OnComponentBeginOverlap(InteractionBox)
  (params (OverlappedComponent :type Primitive%20Component%20Object%20Reference) (OtherActor :type Actor%20Object%20Reference) (OtherComp :type Primitive%20Component%20Object%20Reference) (OtherBodyIndex :type Integer) (bFromSweep :type Boolean) (SweepResult :type Hit%20Result%20Structure%20%28by%20ref%29))
  (bind _asthird_person_character (Utilities|Casting|CastToThirdPersonCharacter OtherActor))
  (Variables|Default|SetPlayerOverlap true))

(event OnComponentEndOverlap(InteractionBox)
  (params (OverlappedComponent :type Primitive%20Component%20Object%20Reference) (OtherActor :type Actor%20Object%20Reference) (OtherComp :type Primitive%20Component%20Object%20Reference) (OtherBodyIndex :type Integer))
  (Utilities|Casting|CastToThirdPersonCharacter OtherActor)
  (Variables|Default|SetPlayerOverlap false))

(event EventBeginPlay
  (Components|Activation|SetActive (Variables|Default|GetRunestoneGlow) false false)
  (bind _newtrack_0 (Timeline|Timeline_0 Play)
    (:Update
      (Class|SceneComponent|AddLocalTransform (Variables|Default|GetSphere) (Math|Transform|MakeTransform _newtrack_0 "0, 0, 0" "1,1,1") false false))))

(event EventTick
  (params (DeltaSeconds :type Float%20%28single-precision%29))
  (if (Variables|Default|GetPlayerOverlap)
    (if (Game|Player|IsInputKeyDown (Game|GetPlayerController 0) "F")
      (if (Variables|/Game/ThirdPersonBP/Blueprints/ThirdPersonCharacter.ThirdPersonCharacter_C|GetStatue2Interacted (stale OnComponentBeginOverlap(InteractionBox) _asthird_person_character))
        (Audio|PlaySoundatLocation "/Game/StarterContent/Audio/Explosion01.Explosion01" (Transformation|GetActorLocation) "0, 0, 0" 1.0 1.0 0.0 0 0 0)
        (if (not (Variables|/Game/ThirdPersonBP/Blueprints/ThirdPersonCharacter.ThirdPersonCharacter_C|GetStatue3Interacted (stale OnComponentBeginOverlap(InteractionBox) _asthird_person_character)))
          (Variables|/Game/ThirdPersonBP/Blueprints/ThirdPersonCharacter.ThirdPersonCharacter_C|SetStatue3Interacted (stale OnComponentBeginOverlap(InteractionBox) _asthird_person_character) true)
          (Components|Activation|SetActive (Variables|Default|GetRunestoneGlow) true true))
        (else
          (Variables|/Game/ThirdPersonBP/Blueprints/ThirdPersonCharacter.ThirdPersonCharacter_C|SetStatue1Interacted (stale OnComponentBeginOverlap(InteractionBox) _asthird_person_character) false)
          (Utilities|FlowControl|Sequence
            (:then_0
              (bind _outactors (Actor|GetAllActorsOfClass "/Game/Assets/Blueprints/Runestone_1.Runestone_1_C"))
              (for _array_element _outactors
                (Components|Activation|SetActive (Variables|/Game/Assets/Blueprints/Runestone_1.Runestone_1_C|GetRunestoneGlow _array_element) false false)))
            (:then_1
              (bind _outactors_2 (Actor|GetAllActorsOfClass "/Game/Assets/Blueprints/Runestone_2.Runestone_2_C"))
              (for _array_element_2 _outactors_2
                (Components|Activation|SetActive (Variables|/Game/Assets/Blueprints/Runestone_2.Runestone_2_C|GetRunestoneGlow _array_element_2) false false)))
            (:then_2
              (bind _outactors_3 (Actor|GetAllActorsOfClass "Runestone_3_C"))
              (for _array_element_3 _outactors_3
                (Components|Activation|SetActive (Variables|Runestone_3_C|GetRunestoneGlow _array_element_3) false false)))
            (:then_3
              (bind _outactors_4 (Actor|GetAllActorsOfClass "/Game/Assets/Blueprints/Runestone_4.Runestone_4_C"))
              (for _array_element_4 _outactors_4
                (Components|Activation|SetActive (Variables|/Game/Assets/Blueprints/Runestone_4.Runestone_4_C|GetRunestoneGlow _array_element_4) false false)))
            (:then_4
              (bind _outactors_5 (Actor|GetAllActorsOfClass "/Game/Assets/Blueprints/Runestone_5.Runestone_5_C"))
              (for _array_element_5 _outactors_5
                (Components|Activation|SetActive (Variables|/Game/Assets/Blueprints/Runestone_5.Runestone_5_C|GetRunestoneGlow _array_element_5) false false)))))))))

(fn ConstructionScript)