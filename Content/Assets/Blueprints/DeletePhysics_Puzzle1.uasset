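; Puzzle 1 trigger box that detects a dropped-in PuzzleHexagon_1 and counts correct placements toward a rabbit destruction cutscene.
; A DoOnce consumed by the first overlap of any actor sets the hexagon's Drop flag and compares its Index to the box's.
; A match increments the Index counter on CameraRig_Blueprint actors.
; At three, timed delays play the CameraRig sequence, add Niagara to DesctructibleRabbit, then hide and destroy it.
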(event OnComponentBeginOverlap(Box)
  (params (OverlappedComponent :type Primitive%20Component%20Object%20Reference) (OtherActor :type Actor%20Object%20Reference) (OtherComp :type Primitive%20Component%20Object%20Reference) (OtherBodyIndex :type Integer) (bFromSweep :type Boolean) (SweepResult :type Hit%20Result%20Structure%20%28by%20ref%29))
  (Utilities|FlowControl|DoOnce false
    (:Completed
      (bind _aspuzzle_hexagon_1 (Utilities|Casting|CastToPuzzleHexagon_1 OtherActor))
      (Variables|/Game/Assets/Blueprints/PuzzleHexagon_1.PuzzleHexagon_1_C|SetDrop _aspuzzle_hexagon_1 true)
      (if (== (Variables|/Game/Assets/Blueprints/PuzzleHexagon_1.PuzzleHexagon_1_C|GetIndex _aspuzzle_hexagon_1) (Variables|Default|GetIndex))
        (bind _outactors (Actor|GetAllActorsOfClass "/Game/Assets/Blueprints/CameraRig_Blueprint.CameraRig_Blueprint_C"))
        (for _array_element _outactors
          (bind _output_get (Variables|/Game/Assets/Blueprints/CameraRig_Blueprint.CameraRig_Blueprint_C|SetIndex _array_element (+ (Variables|/Game/Assets/Blueprints/CameraRig_Blueprint.CameraRig_Blueprint_C|GetIndex _array_element) 1)))
          (if (== _output_get 3)
            (Utilities|FlowControl|Delay 1.0)
            (bind _returnvalue (Sequencer|Player|CreateLevelSequencePlayer "/Game/Assets/Rigs/CameraRig.CameraRig"))
            (Sequencer|Player|Play _returnvalue :!class /Script/MovieScene.MovieSceneSequencePlayer)
            (Utilities|FlowControl|Delay 2.5)
            (bind _returnvalue_2 (Actor|GetActorOfClass "/Game/Assets/Blueprints/DesctructibleRabbit.DesctructibleRabbit_C"))
            (AddComponent|AddNiagaraComponent _returnvalue_2 false)
            (Rendering|SetVisibility (Variables|/Script/Engine.Actor|GetRootComponent _returnvalue_2) false true)
            (Utilities|FlowControl|Delay 2.0)
            (Actor|DestroyActor _returnvalue_2)))))))

(event EventBeginPlay)

(fn ConstructionScript)