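; Interactable runestone actor that the player activates with the F key to mark Statue1Interacted on the ThirdPersonCharacter.
; Overlap events on InteractionBox cache the character and set a flag, which Tick checks while polling the key.
; The collapse sound plays every tick F is held in range, while the glow and character flag are set only once.
; On BeginPlay the glow is switched off and a timeline starts moving the Sphere.
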(event OnComponentBeginOverlap(InteractionBox)
  (params (OverlappedComponent :type Primitive%20Component%20Object%20Reference) (OtherActor :type Actor%20Object%20Reference) (OtherComp :type Primitive%20Component%20Object%20Reference) (OtherBodyIndex :type Integer) (bFromSweep :type Boolean) (SweepResult :type Hit%20Result%20Structure%20%28by%20ref%29))
  (bind _asthird_person_character (Utilities|Casting|CastToThirdPersonCharacter OtherActor))
  (Variables|Default|SetPlayerOverlap true))

(event OnComponentEndOverlap(InteractionBox)
  (params (OverlappedComponent :type Primitive%20Component%20Object%20Reference) (OtherActor :type Actor%20Object%20Reference) (OtherComp :type Primitive%20Component%20Object%20Reference) (OtherBodyIndex :type Integer))
  (Utilities|Casting|CastToThirdPersonCharacter OtherActor)
  (Variables|Default|SetPlayerOverlap false))

(event EventBeginPlay
  (Components|Activation|SetActive (Variables|Default|GetRunestoneGlow) false false)
  (bind _newtrack_0 (Timeline|Timeline_0 Play)
    (:Update
      (Class|SceneComponent|AddLocalTransform (Variables|Default|GetSphere) (Math|Transform|MakeTransform _newtrack_0 "0, 0, 0" "1,1,1") false false))))

(event EventTick
  (params (DeltaSeconds :type Float%20%28single-precision%29))
  (if (Variables|Default|GetPlayerOverlap)
    (if (Game|Player|IsInputKeyDown (Game|GetPlayerController 0) "F")
      (Audio|PlaySoundatLocation "/Game/StarterContent/Audio/Collapse01.Collapse01" (Transformation|GetActorLocation) "0, 0, 0" 1.0 1.0 0.0 0 0 0)
      (if (not (Variables|/Game/ThirdPersonBP/Blueprints/ThirdPersonCharacter.ThirdPersonCharacter_C|GetStatue1Interacted (stale OnComponentBeginOverlap(InteractionBox) _asthird_person_character)))
        (Variables|/Game/ThirdPersonBP/Blueprints/ThirdPersonCharacter.ThirdPersonCharacter_C|SetStatue1Interacted (stale OnComponentBeginOverlap(InteractionBox) _asthird_person_character) true)
        (Components|Activation|SetActive (Variables|Default|GetRunestoneGlow) true true)))))

(fn ConstructionScript)